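; BP_Projectile_Good_Medium is a beneficial projectile that heals the side-scroller player on contact.
; On BeginPlay, its physics Sphere gets a fixed downward velocity along Z.
; When the Sphere overlaps a SideScrollerCharacter, it adds a small amount to PlayerHealth, capped at full, then destroys itself.
; The graph comment mentions reversing velocity on umbrella hits, but this graph contains no such logic.
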(event `self.ReceiveBeginPlay`
  ;[1 1 1] sets movement speed for the projectile on the z axis and when it hits the umbrella reverses that value.
  (`PrimitiveComponent.SetPhysicsLinearVelocity` (`self.Sphere`) (0.0 0.0 -400.0) false "None"))

(event `self.Sphere.OnComponentBeginOverlap`
  (params (OverlappedComponent :type "PrimitiveComponent Object Reference") (OtherActor :type "Actor Object Reference") (OtherComp :type "PrimitiveComponent Object Reference") (OtherBodyIndex :type Integer) (bFromSweep :type Boolean) (SweepResult :type "HitResult Structure (by ref)"))
  (bind _asside_scroller_character (cast `/Game/SideScrollerBP/Blueprints/SideScrollerCharacter` OtherActor))
  (bind _returnvalue (+ (`/Game/SideScrollerBP/Blueprints/SideScrollerCharacter.PlayerHealth` _asside_scroller_character) 0.1))
  (if (>= _returnvalue 1.0)
    (set `/Game/SideScrollerBP/Blueprints/SideScrollerCharacter.PlayerHealth` 1.0 _asside_scroller_character)
    (else
      (set `/Game/SideScrollerBP/Blueprints/SideScrollerCharacter.PlayerHealth` _returnvalue _asside_scroller_character)))
  (`self.K2_DestroyActor`))

(fn `UserConstructionScript`)