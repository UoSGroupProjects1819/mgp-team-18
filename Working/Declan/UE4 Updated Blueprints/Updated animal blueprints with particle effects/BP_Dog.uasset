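; BP_Dog is a wandering dog pickup that a SideScrollerCharacter collects by touch.
; From BeginPlay it loops every half second, setting the ProjectileMovement velocity to a random Y and Z within speed limits while X stays zero.
; Overlapping Sphere1 with the character increments its DogCount, prints the new count and destroys the dog.
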(event `self.Sphere1.OnComponentBeginOverlap`
  (params (OverlappedComponent :type "PrimitiveComponent Object Reference") (OtherActor :type "Actor Object Reference") (OtherComp :type "PrimitiveComponent Object Reference") (OtherBodyIndex :type Integer) (bFromSweep :type Boolean) (SweepResult :type "HitResult Structure (by ref)"))
  (bind _asside_scroller_character (cast `/Game/SideScrollerBP/Blueprints/SideScrollerCharacter` OtherActor))
  (bind _output_get (set `/Game/SideScrollerBP/Blueprints/SideScrollerCharacter.Dog_Count` (+ (`/Game/SideScrollerBP/Blueprints/SideScrollerCharacter.Dog_Count` _asside_scroller_character) 1) _asside_scroller_character))
  (`KismetSystemLibrary.PrintString` (`KismetStringLibrary.Conv_IntToString` _output_get))
  (`self.K2_DestroyActor`))

(event `self.ReceiveBeginPlay`
  (set `MovementComponent.Velocity` (`KismetMathLibrary.MakeVector` 0.0 (`KismetMathLibrary.RandomFloatInRange` (`self.Speed_MinY`) (`self.Speed_MaxY`)) (`KismetMathLibrary.RandomFloatInRange` (`self.Speed_MinZ`) (`self.Speed_MaxZ`))) (`self.ProjectileMovement`) :!label _label)
  (`KismetSystemLibrary.Delay` 0.5)
  (goto _label))

(fn `UserConstructionScript`)