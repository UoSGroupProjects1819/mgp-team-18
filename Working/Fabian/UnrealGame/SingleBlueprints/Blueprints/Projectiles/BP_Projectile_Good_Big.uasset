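; BP_Projectile_Good_Big is a falling pickup that restores a small amount of the player's health.
; On BeginPlay its physics Sphere is given a fixed downward velocity.
; Overlapping BP_UmbrellaV2 inverts the Sphere's vertical velocity, deflecting the projectile.
; When the Sphere overlaps the SideScrollerCharacter, it adds to PlayerHealth, capped at full, then destroys itself.
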(event `self.ReceiveBeginPlay`
  (`PrimitiveComponent.SetPhysicsLinearVelocity` (`self.Sphere`) (0.0 0.0 -400.0) false "None"))

(event `self.ReceiveActorBeginOverlap`
  (params (OtherActor :type "Actor Object Reference"))
  (cast `/Game/SideScrollerBP/Blueprints/BP_UmbrellaV2` OtherActor)
  (bind _returnvalue (`PrimitiveComponent.GetPhysicsLinearVelocity` (`self.Sphere`) "None"))
  (`PrimitiveComponent.SetPhysicsLinearVelocity` (`self.Sphere`) (`KismetMathLibrary.MakeVector` (.x _returnvalue) (.y _returnvalue) (* (.z _returnvalue) -1.0)) false "None"))

(event `self.Sphere.OnComponentBeginOverlap`
  (params (OverlappedComponent :type "PrimitiveComponent Object Reference") (OtherActor :type "Actor Object Reference") (OtherComp :type "PrimitiveComponent Object Reference") (OtherBodyIndex :type Integer) (bFromSweep :type Boolean) (SweepResult :type "HitResult Structure (by ref)"))
  (bind _asside_scroller_character (cast `/Game/SideScrollerBP/Blueprints/SideScrollerCharacter` OtherActor))
  (bind _returnvalue (+ (`/Game/SideScrollerBP/Blueprints/SideScrollerCharacter.PlayerHealth` _asside_scroller_character) 0.05))
  (if (>= _returnvalue 1.0)
    (set `/Game/SideScrollerBP/Blueprints/SideScrollerCharacter.PlayerHealth` 1.0 _asside_scroller_character)
    (else
      (set `/Game/SideScrollerBP/Blueprints/SideScrollerCharacter.PlayerHealth` _returnvalue _asside_scroller_character)))
  (`self.K2_DestroyActor`))

(fn `UserConstructionScript`)