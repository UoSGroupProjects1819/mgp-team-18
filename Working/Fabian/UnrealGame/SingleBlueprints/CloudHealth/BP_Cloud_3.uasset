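; Enemy cloud for a side-scroller that rains, spawns projectiles and animals, and can be shot down.
; While active, it spawns weighted-random child actors in SpawnBox at random intervals; a player overlapping AnimalTrigger adds a random animal, up to a limit.
; Big, medium and small bad-projectile hits subtract different amounts of CloudHealth, destroying the cloud with an explosion at zero.
; Tick pushes CloudHealth to the widget health bar.
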(event `self.ReceiveBeginPlay`
  ;[1 1 1] Comment
  (`GameplayStatics.SpawnEmitterAttached` "/Game/ParticleEffects/Rain/RainfallC3_P.RainfallC3_P" (`self.Cloud3`) "None" (130.0 0.0 15.0) (struct :`Yaw` 90.0))
  (if (`self.CloudActive`) :!label _label
    (`KismetSystemLibrary.Delay` (`KismetMathLibrary.RandomFloatInRange` 0.5 1.5))
    (`self.Spawn_Projectile`)
    (goto _label)))

(event `self.AnimalTrigger.OnComponentBeginOverlap`
  (params (OverlappedComponent :type "PrimitiveComponent Object Reference") (OtherActor :type "Actor Object Reference") (OtherComp :type "PrimitiveComponent Object Reference") (OtherBodyIndex :type Integer) (bFromSweep :type Boolean) (SweepResult :type "HitResult Structure (by ref)"))
  ;[1 1 1] Comment
  (cast `/Game/SideScrollerBP/Blueprints/SideScrollerCharacter` OtherActor)
  (`self.Spawn_Animal`))

(event `self.CloudHitbox.OnComponentBeginOverlap`
  (params (OverlappedComponent :type "PrimitiveComponent Object Reference") (OtherActor :type "Actor Object Reference") (OtherComp :type "PrimitiveComponent Object Reference") (OtherBodyIndex :type Integer) (bFromSweep :type Boolean) (SweepResult :type "HitResult Structure (by ref)"))
  ;[1 1 1] Comment
  (`|ExecutionSequence`
    (:`then_0`
      (cast `/Game/SideScrollerBP/Blueprints/BP_Projectile_Bad_Big` OtherActor)
      (bind _output_get (set `self.CloudHealth` (- (`self.CloudHealth`) 0.5)))
      (`/Engine/EditorBlueprintResources/StandardMacros.CompareFloat` _output_get
        (:`>`
          (`KismetSystemLibrary.PrintString` "hit"))
        (:`==`
          (`KismetSystemLibrary.PrintString` "destroyed" :!label _label_2)
          (`self.K2_DestroyActor` (`ActorComponent.GetOwner` (`self.Cloud3`)))
          (`GameplayStatics.SpawnEmitterAtLocation` "/Game/CartoonFX2/Particles/PS_Explosion.PS_Explosion" (`self.K2_GetActorLocation`) :!label _label_3))
        (:`<`
          (goto _label_2))))
    (:`then_1`
      (cast `/Game/SideScrollerBP/Blueprints/BP_Projectile_Bad_Medium` OtherActor)
      (bind _output_get_2 (set `self.CloudHealth` (- (`self.CloudHealth`) 0.1)))
      (`/Engine/EditorBlueprintResources/StandardMacros.CompareFloat` _output_get_2
        (:`>`
          (`KismetSystemLibrary.PrintString` "hit"))
        (:`==`
          (`KismetSystemLibrary.PrintString` "destroyed" :!label _label_4)
          (`self.K2_DestroyActor` (`ActorComponent.GetOwner` (`self.Cloud3`)))
          (goto _label_3))
        (:`<`
          (goto _label_4))))
    (:`then_2`
      (cast `/Game/SideScrollerBP/Blueprints/BP_Projectile_Bad_Small` OtherActor)
      (bind _output_get_3 (set `self.CloudHealth` (- (`self.CloudHealth`) 0.05)))
      (`/Engine/EditorBlueprintResources/StandardMacros.CompareFloat` _output_get_3
        (:`>`
          (`KismetSystemLibrary.PrintString` "hit"))
        (:`==`
          (`KismetSystemLibrary.PrintString` "destroyed" :!label _label_5)
          (`self.K2_DestroyActor` (`ActorComponent.GetOwner` (`self.Cloud3`)))
          (goto _label_3))
        (:`<`
          (goto _label_5))))))

(event `self.ReceiveTick`
  (params (DeltaSeconds :type "Float (single-precision)"))
  ;[1 1 1] Comment
  (bind _asenemy_health_ui (cast `/Game/SideScrollerBP/HUD/EnemyHealthUI` (`WidgetComponent.GetUserWidgetObject` (`self.Widget`))))
  (`ProgressBar.SetPercent` (`/Game/SideScrollerBP/HUD/EnemyHealthUI.ProgressBar_114` _asenemy_health_ui) (`self.CloudHealth`)))

(fn `Spawn_Animal`
  (bind _spawnbox (`self.SpawnBox`))
  (bind _returnvalue (`KismetMathLibrary.Conv_VectorToTransform` (`KismetMathLibrary.RandomPointInBoundingBox` (`SceneComponent.RelativeLocation` _spawnbox) (`BoxComponent.BoxExtent` _spawnbox))))
  (if (`self.CloudActive`)
    (if (< (`self.Animal_Counter`) (`self.Animal_Counter_Limit`))
      (switch `int` (`KismetMathLibrary.RandomIntegerInRange` 0 4)
        (:`0`
          (`AddComponent|NODE_AddChildActorComponent-2` :`RelativeTransform` _returnvalue))
        (:`1`
          (`AddComponent|NODE_AddChildActorComponent-4` :`RelativeTransform` _returnvalue))
        (:`2`
          (`AddComponent|NODE_AddChildActorComponent-3` :`RelativeTransform` _returnvalue))
        (:`3`
          (`AddComponent|NODE_AddChildActorComponent-5` :`RelativeTransform` _returnvalue))
        (:`4`
          (`AddComponent|NODE_AddChildActorComponent-6` :`RelativeTransform` _returnvalue)))
      (set `self.Animal_Counter` (+ (`self.Animal_Counter`) 1)))))

(fn `Spawn_Projectile`
  (bind _spawnbox (`self.SpawnBox`))
  (bind _returnvalue (`KismetMathLibrary.Conv_VectorToTransform` (`KismetMathLibrary.RandomPointInBoundingBox` (`SceneComponent.RelativeLocation` _spawnbox) (`BoxComponent.BoxExtent` _spawnbox))))
  (if (`self.CloudActive`)
    (switch `int` (`KismetMathLibrary.RandomIntegerInRange` 0 2)
      (:`0`
        (switch `int` (`KismetMathLibrary.RandomIntegerInRange` 0 5) :!label _label
          (:`0`
            (`AddComponent|NODE_AddChildActorComponent-11` :`RelativeTransform` _returnvalue :!label _label_2))
          (:`1`
            (goto _label_2))
          (:`2`
            (`AddComponent|NODE_AddChildActorComponent-7` :`RelativeTransform` _returnvalue :!label _label_3))
          (:`3`
            (goto _label_3))
          (:`4`
            (goto _label_3))
          (:`5`
            (`AddComponent|NODE_AddChildActorComponent-12` :`RelativeTransform` _returnvalue))))
      (:`1`
        (goto _label))
      (:`2`
        (switch `int` (`KismetMathLibrary.RandomIntegerInRange` 0 2)
          (:`0`
            (`AddComponent|NODE_AddChildActorComponent-9` :`RelativeTransform` _returnvalue))
          (:`1`
            (`AddComponent|NODE_AddChildActorComponent-8` :`RelativeTransform` _returnvalue))
          (:`2`
            (`AddComponent|NODE_AddChildActorComponent-10` :`RelativeTransform` _returnvalue)))))))

(fn `UserConstructionScript`)